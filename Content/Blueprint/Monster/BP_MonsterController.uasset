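; AI controller for the monster that runs BT_Monster and feeds it player sightings from AI Perception.
; Sensing a living player sets SeesPlayer and stores player 0's location and actor as TargetLocation and TargetActor in the Blackboard.
; A chase cue plays on the pawn only when SeesPlayer was previously false.
; Lost stimuli, dead players or non-player targets clear only SeesPlayer, leaving the last stored target in place.
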(event OnTargetPerceptionInfoUpdated(AIPerception)
  (params (UpdateInfo :type Actor%20Perception%20Update%20Info%20Structure%20%28by%20ref%29))
  (bind (_targetid _target _stimulus) (Utilities|Struct|BreakActorPerceptionUpdateInfo UpdateInfo))
  (bind _returnvalue (Utilities|Name|MakeLiteralName "SeesPlayer"))
  (bind _returnvalue_2 (Game|GetPlayerCharacter 0))
  (bind _blackboard (Variables|Default|GetBlackboard))
  (bind _asbp_player_character (Utilities|Casting|CastToBP_PlayerCharacter _target)
    (:then
      (if (Variables|/Game/Blueprint/Player/BP_PlayerCharacter.BP_PlayerCharacter_C|GetbIsAlive _asbp_player_character)
        (if (.bSuccessfullySensed (Utilities|Struct|BreakAIStimulus _stimulus))
          (if (ScalableFloat|GetValueasBool (Variables|Default|GetBlackboard) (Utilities|Name|MakeLiteralName "SeesPlayer"))
            _
            (else
              (Audio|SpawnSoundAttached "/Game/Audio/SFX/Monster/Cue_Monster_Chase.Cue_Monster_Chase" (Variables|/Script/Engine.Actor|GetRootComponent (Pawn|GetControlledPawn)) "None" "0, 0, 0" "0, 0, 0" "KeepRelativeOffset" false 1.0 1.0 0.0 0 0)
              (AI|Components|Blackboard|SetValueasBool _blackboard _returnvalue true)))
          (AI|Components|Blackboard|SetValueasVector _blackboard (Utilities|Name|MakeLiteralName "TargetLocation") (Transformation|GetActorLocation _returnvalue_2))
          (AI|Components|Blackboard|SetValueasObject _blackboard (Utilities|Name|MakeLiteralName "TargetActor") _returnvalue_2)
          (else
            (AI|Components|Blackboard|SetValueasBool _blackboard _returnvalue false :!label _label)))
        (else
          (goto _label))))
    (:CastFailed
      (goto _label))))

(event EventBeginPlay
  (AI|RunBehaviorTree "/Game/Blueprint/Monster/AI/BT_Monster.BT_Monster"))

(event EventTick
  (params (DeltaSeconds :type Float%20%28single-precision%29)))

(fn ConstructionScript)