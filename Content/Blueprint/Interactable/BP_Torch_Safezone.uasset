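; Interactable torch that the player lights with oil to create a temporary safe zone that stops the monster.
; Use spends oil, starts the flame, disables the highlight, and stops the monster if already within the radius; later sphere overlaps stop it while lit.
; A looping timer drains FillState over BurnTime into the Niagara flame's spawn parameter, then resets the torch and resumes the monster.
; The construction script sizes the sphere from SafeZoneRadius.
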(event OnComponentBeginOverlap(SafeZone)
  (params (OverlappedComponent :type Primitive%20Component%20Object%20Reference) (OtherActor :type Actor%20Object%20Reference) (OtherComp :type Primitive%20Component%20Object%20Reference) (OtherBodyIndex :type Integer) (bFromSweep :type Boolean) (SweepResult :type Hit%20Result%20Structure%20%28by%20ref%29))
  (if (Variables|Default|GetbIsActive)
    (bind _asbp_monster (Utilities|Casting|CastToBP_Monster OtherActor))
    (Default|Stop _asbp_monster self)))

(event Custom|BurnTorch
  (Effects|Components|ParticleSystem|SetFloatParameter (Variables|Default|GetFlame) "FlameSpawn" (Variables|Default|GetFillState))
  (if (> (Variables|Default|GetFillState) 0.0)
    (Variables|Default|SetFillState (- (Variables|Default|GetFillState) (/ 1.0 (/ (Variables|GameplayLogic|GetBurnTime) 0.2))))
    (else
      (Variables|Default|SetbIsActive false)
      (Utilities|Time|ClearandInvalidateTimerbyHandle (Variables|Default|GetTimerHandleTorch))
      (Variables|Default|SetFillState 1.0)
      (Variables|/Script/Engine.ActorComponent|SetComponentTags (Variables|Default|GetStaticMesh) (Utilities|Array|MakeArray "highlightable"))
      (Components|Activation|SetActive (Variables|Default|GetFlame) false true)
      (Default|Resume (Variables|Default|GetMonster)))))

(event EventUse
  (bind _staticmesh (Variables|Default|GetStaticMesh))
  (if (and (> (Variables|/Game/Blueprint/Player/BP_PlayerCharacter.BP_PlayerCharacter_C|GetOil (Variables|Default|GetPlayer)) 0.0) (not (Variables|Default|GetbIsActive)))
    (Components|Activation|SetActive (Variables|Default|GetFlame) true true)
    (Variables|Default|SetbIsActive true)
    (Variables|/Script/Engine.ActorComponent|SetComponentTags _staticmesh (Utilities|Array|MakeArray "None"))
    (Rendering|SetRenderCustomDepth _staticmesh false)
    (Default|ChangeOil (Variables|Default|GetPlayer) -1e+01 true)
    (Utilities|FlowControl|Sequence
      (:then_0
        (if (<= (Transformation|GetDistanceTo (Variables|Default|GetMonster) self) (Variables|GameplayLogic|GetSafeZoneRadius))
          (Default|Stop (Variables|Default|GetMonster) self)))
      (:then_1
        (bind _returnvalue (Utilities|Time|SetTimerbyEvent (delegate Custom|BurnTorch) 0.2 true))
        (Variables|Default|SetTimerHandleTorch _returnvalue)))))

(event EventBeginPlay
  (bind _asbp_player_character (Utilities|Casting|CastToBP_PlayerCharacter (Game|GetPlayerCharacter 0)))
  (Variables|Default|SetPlayer _asbp_player_character)
  (bind _returnvalue (Actor|GetActorOfClass "/Game/Blueprint/Monster/BP_Monster.BP_Monster_C"))
  (Variables|Default|SetMonster _returnvalue))

(fn ConstructionScript
  (Components|Sphere|SetSphereRadius (Variables|Default|GetSafeZone) (Variables|GameplayLogic|GetSafeZoneRadius) true))