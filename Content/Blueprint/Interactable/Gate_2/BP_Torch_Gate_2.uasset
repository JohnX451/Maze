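; BP_Torch_Gate_2 is a Gate 2 puzzle torch whose lit state can be toggled by another torch, noted as the center one.
; ZoneEntered activates the flame, then plays ignition and enables audio for active torches or hides the flame for inactive ones.
; ToggleFromOtherTorch calls ToggleFlame, which flips visibility and IsActive.
; Extinguishing plays a sound and stops the audio, while relighting only unhides the flame.
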(event Custom|Toggle%20From%20Other%20Torch
  ;[1 1 1] Event if the Torch is affected by the center torch and needs to be toggled
  (CallFunction|ToggleFlame (Variables|Default|GetFlame) (Variables|Default|GetbIsActive)))

(event Custom|Zone%20Entered
  ;[1 1 1] Activate Torches when Player enters Zone. Set Flame to hidden except for specific active torches.
  (Components|Activation|SetActive (Variables|Default|GetFlame) true true)
  (if (Variables|Default|GetbIsActive)
    (Audio|SpawnSoundAttached "/Game/Audio/SFX/Fire/Cue_Torch_Ignite.Cue_Torch_Ignite" (Variables|Default|GetFlame) "None" "0, 0, 0" "0, 0, 0" "KeepRelativeOffset" false 1.0 1.0 0.0 0 0)
    (Components|Activation|SetActive (Variables|Default|GetAudio) true true)
    (else
      (Development|SetHiddeninGame (Variables|Default|GetFlame) true false))))

(event EventBeginPlay
  (bind _asbp_player_character (Utilities|Casting|CastToBP_PlayerCharacter (Game|GetPlayerCharacter 0)))
  (Variables|Default|SetPlayer _asbp_player_character))

(fn ConstructionScript)

(fn ToggleFlame
  (params (Flame :type Scene%20Component%20Object%20Reference) (CurrentState :type Boolean))
  (Development|SetHiddeninGame Flame CurrentState false)
  (bind _output_get (Variables|Default|SetbIsActive (not CurrentState)))
  (if (not _output_get)
    (Audio|SpawnSoundAttached "/Game/Audio/SFX/Fire/Cue_Lantern_Extinguish.Cue_Lantern_Extinguish" (Variables|Default|GetFlame) "None" "0, 0, 0" "0, 0, 0" "KeepRelativeOffset" false 1.0 1.0 0.0 0 0)
    (Components|Activation|SetActive (Variables|Default|GetAudio) false true)))