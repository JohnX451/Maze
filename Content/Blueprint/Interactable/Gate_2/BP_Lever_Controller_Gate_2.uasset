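; Lever puzzle controller for Gate 2 that opens the gate when five levers are activated in a fixed order.
; LeverActivated uses nested stage flags to compare each lever with the expected one, clearing SequenceCorrect on a mismatch.
; EvaluateLevers counts activations and, on the fifth, opens the Gate or tells TorchController to turn off a torch.
; Failure resets the count and SequenceCorrect, but leaves stage flags set.
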(event Custom|Lever%20Activated
  (params (Lever :type BP%20Lever%20Gate%202%20Object%20Reference))
  (if (Variables|Default|GetSequenceCorrect)
    (if (Variables|Default|GetFirstLeverSet)
      (if (Variables|Default|GetSecondLeverSet)
        (if (Variables|Default|GetThirdLeverSet)
          (if (Variables|Default|GetFourthLeverSet)
            (bind _isequal (CallFunction|CheckifLeversEqual Lever (Variables|Levers|GetLever%203)))
            (if _isequal
              (Variables|Default|SetFifthLeverSet true)
              (else
                (Variables|Default|SetSequenceCorrect false)))
            (else
              (bind _isequal_2 (CallFunction|CheckifLeversEqual Lever (Variables|Levers|GetLever%201)))
              (if _isequal_2
                (Variables|Default|SetFourthLeverSet true)
                (else
                  (Variables|Default|SetSequenceCorrect false)))))
          (else
            (bind _isequal_3 (CallFunction|CheckifLeversEqual Lever (Variables|Levers|GetLever%205)))
            (if _isequal_3
              (Variables|Default|SetThirdLeverSet true)
              (else
                (Variables|Default|SetSequenceCorrect false)))))
        (else
          (bind _isequal_4 (CallFunction|CheckifLeversEqual Lever (Variables|Levers|GetLever%204)))
          (if _isequal_4
            (Variables|Default|SetSecondLeverSet true)
            (else
              (Variables|Default|SetSequenceCorrect false)))))
      (else
        (bind _isequal_5 (CallFunction|CheckifLeversEqual Lever (Variables|Levers|GetLever%202)))
        (if _isequal_5
          (Variables|Default|SetFirstLeverSet true)
          (else
            (Variables|Default|SetSequenceCorrect false)))))
    (CallFunction|EvaluateLevers)
    (else
      (CallFunction|EvaluateLevers))))

(event EventBeginPlay)

(event Collision|EventActorBeginOverlap
  (params (OtherActor :type Actor%20Object%20Reference)))

(event EventTick
  (params (DeltaSeconds :type Float%20%28single-precision%29)))

(fn ConstructionScript)

(fn EvaluateLevers
  (Math|Integer|IncrementInt (Variables|Default|GetNumber%20of%20Levers%20Activated)
    (:%20%20
      (if (== 5 (Variables|Default|GetNumber%20of%20Levers%20Activated))
        (if (Variables|Default|GetSequenceCorrect)
          (Default|OpenGate (Variables|Gameplay|GetGate))
          (else
            (Default|TurnOffNextTorch (Variables|Gameplay|GetTorchController))
            (Variables|Default|SetNumber%20of%20Levers%20Activated 0)
            (Variables|Default|SetSequenceCorrect true)))))))

(fn CheckifLeversEqual
  (params (InputLever :type Object%20Object%20Reference) (StageLever :type BP%20Lever%20Gate%202%20Object%20Reference))
  (return (== InputLever StageLever)))