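; BP_Stone_Row is a puzzle row of three stepping stones in which only the one at StableIndex holds.
; The construction script gives each stone a random quarter-turn yaw and places an Arrow above the stable stone.
; The player's first Hitbox overlap, after a short delay, breaks the other stones with effects and physics simulation.
; ShowHint marks the stable stone with sparks and a help sound.
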(event OnComponentBeginOverlap(Hitbox)
  (params (OverlappedComponent :type Primitive%20Component%20Object%20Reference) (OtherActor :type Actor%20Object%20Reference) (OtherComp :type Primitive%20Component%20Object%20Reference) (OtherBodyIndex :type Integer) (bFromSweep :type Boolean) (SweepResult :type Hit%20Result%20Structure%20%28by%20ref%29))
  (Utilities|Casting|CastToBP_PlayerCharacter OtherActor)
  (Utilities|FlowControl|DoOnce false
    (:Completed
      (Utilities|FlowControl|Delay 0.1)
      (for (_array_element _array_index) (Variables|Default|GetStones)
        (if (!= _array_index (Variables|Default|GetStableIndex))
          (CallFunction|DestroyTile _array_element))))))

(event Custom|ShowHint
  (bind _stones (Variables|Default|GetStones))
  (bind _stableindex (Variables|Default|GetStableIndex))
  (bind _output (Utilities|Array|Get(acopy) _stones _stableindex))
  (bind _returnvalue (Transformation|GetWorldLocation _output))
  (bind _returnvalue_2 (+ _returnvalue "0.000000,0.000000,20.000000"))
  (Effects|SpawnEmitteratLocation "/Game/ThirdParty/Realistic_Starter_VFX_Pack_Vol2/Particles/Sparks/P_Sparks_C.P_Sparks_C" _returnvalue_2)
  (Audio|SpawnSoundatLocation "/Game/Audio/SFX/Puzzles/Cue_Puzzle_Help.Cue_Puzzle_Help" _returnvalue_2 "0, 0, 0" 1.0 1.0 0.0 0 0))

(fn ConstructionScript
  (Variables|Default|SetStones (Utilities|Array|MakeArray (Variables|Stones|GetStone_Left) (Variables|Stones|GetStone_Middle) (Variables|Stones|GetStone_Right)))
  (CallFunction|SetUpTile))

(fn SetUpTile
  (for (_array_element _array_index) (Variables|Default|GetStones)
    (Transformation|SetRelativeRotation _array_element (Math|Rotator|MakeRotator 0.0 0.0 (Utilities|Select :Index (Math|Random|RandomIntegerinRange 0 3) :Option%200 0.0 :Option%201 9e+01 :Option%202 -9e+01 :Option%203 1.8e+02)) false false)
    (if (== (Variables|Default|GetStableIndex) _array_index)
      (Transformation|SetWorldLocation (Variables|Default|GetArrow) (Math|Vector|MakeVector (.x (Transformation|GetWorldLocation _array_element)) (.y (Transformation|GetWorldLocation _array_element)) (+ (.z (Transformation|GetWorldLocation _array_element)) 2e+01)) false false))))

(fn DestroyTile
  (params (Tile :type Static%20Mesh%20Component%20Object%20Reference))
  (Effects|SpawnEmitteratLocation "/Game/ThirdParty/Realistic_Starter_VFX_Pack_Vol2/Particles/Destruction/P_Destruction_Concrete.P_Destruction_Concrete" (Transformation|GetWorldLocation Tile))
  (Audio|SpawnSoundAttached "/Game/Audio/SFX/Puzzles/Cue_Tile_Break.Cue_Tile_Break" Tile "None" "0, 0, 0" "0, 0, 0" "KeepRelativeOffset" false 1.0 1.0 0.0 0 0)
  (Physics|SetSimulatePhysics Tile true))