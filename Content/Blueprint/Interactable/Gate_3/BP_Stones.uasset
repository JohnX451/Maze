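; BP_Stones is a Gate 3 interactable with three stones, each either stationary or falling, and a flame for each.
; A hitbox overlap briefly delays, then enables physics on non-stationary stones.
; ToggleFlame and TurnoffFlame events toggle or hide flames for stationary stones only.
; The construction script hides all flames and gives each stone a random quarter-turn yaw.
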(event OnComponentBeginOverlap(Hitbox)
  (params (OverlappedComponent :type Primitive%20Component%20Object%20Reference) (OtherActor :type Actor%20Object%20Reference) (OtherComp :type Primitive%20Component%20Object%20Reference) (OtherBodyIndex :type Integer) (bFromSweep :type Boolean) (SweepResult :type Hit%20Result%20Structure%20%28by%20ref%29))
  (Utilities|FlowControl|Delay 0.1)
  (if (Variables|Default|GetStoneLeftStationary)
    _
    (else
      (Physics|SetSimulatePhysics (Variables|Stones|GetStone_Left) true)))
  (if (Variables|Default|GetStoneMiddleStationary)
    _
    (else
      (Physics|SetSimulatePhysics (Variables|Stones|GetStone_Middle) true)))
  (if (not (Variables|Default|GetStoneRightStationary))
    (Physics|SetSimulatePhysics (Variables|Stones|GetStone_Right) true)))

(event Custom|Toggle%20Flame
  (bind _flame_right (Variables|Default|GetFlame_Right))
  (bind _flame_middle (Variables|Default|GetFlame_Middle))
  (bind _flame_left (Variables|Default|GetFlame_Left))
  (if (Variables|Default|GetStoneRightStationary)
    (Development|SetHiddeninGame _flame_right (not (Variables|/Script/Engine.SceneComponent|GetbHiddenInGame _flame_right)) false))
  (if (Variables|Default|GetStoneMiddleStationary)
    (Development|SetHiddeninGame _flame_middle (not (Variables|/Script/Engine.SceneComponent|GetbHiddenInGame _flame_middle)) false))
  (if (Variables|Default|GetStoneLeftStationary)
    (Development|SetHiddeninGame _flame_left (not (Variables|/Script/Engine.SceneComponent|GetbHiddenInGame _flame_left)) false)))

(event Custom|Turn%20off%20Flame
  (if (Variables|Default|GetStoneRightStationary)
    (Development|SetHiddeninGame (Variables|Default|GetFlame_Right) true false))
  (if (Variables|Default|GetStoneMiddleStationary)
    (Development|SetHiddeninGame (Variables|Default|GetFlame_Middle) true false))
  (if (Variables|Default|GetStoneLeftStationary)
    (Development|SetHiddeninGame (Variables|Default|GetFlame_Left) true false)))

(event EventBeginPlay)

(event Collision|EventActorBeginOverlap
  (params (OtherActor :type Actor%20Object%20Reference)))

(event EventTick
  (params (DeltaSeconds :type Float%20%28single-precision%29)))

(fn ConstructionScript
  (Development|SetHiddeninGame (Variables|Default|GetFlame_Right) true false)
  (Development|SetHiddeninGame (Variables|Default|GetFlame_Middle) true false)
  (Development|SetHiddeninGame (Variables|Default|GetFlame_Left) true false)
  (CallFunction|SetUpRotation))

(fn SetUpRotation
  (for _array_element (Utilities|Array|MakeArray (Variables|Stones|GetStone_Left) (Variables|Stones|GetStone_Middle) (Variables|Stones|GetStone_Right))
    (Transformation|SetRelativeRotation _array_element (Math|Rotator|MakeRotator 0.0 0.0 (Utilities|Select :Index (Math|Random|RandomIntegerinRange 0 3) :Option%200 0.0 :Option%201 9e+01 :Option%202 -9e+01 :Option%203 1.8e+02)) false false)))