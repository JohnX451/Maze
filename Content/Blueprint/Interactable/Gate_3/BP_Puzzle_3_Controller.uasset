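; Puzzle controller for Gate 3 that plays a repeating hint sequence across five stones.
; The construction script gathers the five stone references into an ordered array.
; StartSequence starts a looping one-second timer that calls ShowHint on the current stone and advances the index, wrapping after the last.
; StopSequence clears the timer and resets the index to the first stone.
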(event Custom|StartSequence
  (bind _returnvalue (Utilities|Time|SetTimerbyEvent (delegate Custom|PlaySequence) 1.0 true))
  (Variables|Default|SetTimerHandle_PuzzleSequence _returnvalue))

(event Custom|PlaySequence
  (Default|ShowHint (Utilities|Array|Get(acopy) (Variables|Default|GetStones) (Variables|Default|GetCurrentIndex)))
  (if (>= (Variables|Default|GetCurrentIndex) 4)
    (Variables|Default|SetCurrentIndex 0)
    (else
      (Math|Integer|IncrementInt (Variables|Default|GetCurrentIndex)))))

(event Custom|StopSequence
  (Utilities|Time|ClearandInvalidateTimerbyHandle (Variables|Default|GetTimerHandle_PuzzleSequence))
  (Variables|Default|SetCurrentIndex 0))

(fn ConstructionScript
  (Variables|Default|SetStones (Utilities|Array|MakeArray (Variables|Stones|GetStones_1) (Variables|Stones|GetStones_2) (Variables|Stones|GetStones_3) (Variables|Stones|GetStones_4) (Variables|Stones|GetStones_5))))