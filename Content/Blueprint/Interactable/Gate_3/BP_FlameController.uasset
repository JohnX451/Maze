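; BP_FlameController is a Gate 3 interactable controller that switches flames on five referenced stones.
; ToggleXStonesFlame takes a stone number, checks it is from 1 to 5, and toggles that stone's flame through a chain of branches.
; TurnoffallFlames calls TurnOffFlame on all five stones.
; It has no active tick, begin play or construction logic and acts only when these events are called.
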(event Custom|Toggle%20X%20Stones%20Flame
  (params (StoneNr :type Integer))
  (if (and (<= StoneNr 5) (>= StoneNr 1))
    (if (== StoneNr 1)
      (Default|ToggleFlame (Variables|Stones|GetStones_1))
      (elif (== StoneNr 2)
        (Default|ToggleFlame (Variables|Stones|GetStones_2))
        (elif (== StoneNr 3)
          (Default|ToggleFlame (Variables|Stones|GetStones_3))
          (elif (== StoneNr 4)
            (Default|ToggleFlame (Variables|Stones|GetStones_4))
            (elif (== StoneNr 5)
              (Default|ToggleFlame (Variables|Stones|GetStones_5)))))))))

(event Custom|Turn%20off%20all%20Flames
  (Default|TurnOffFlame (Variables|Stones|GetStones_1))
  (Default|TurnOffFlame (Variables|Stones|GetStones_2))
  (Default|TurnOffFlame (Variables|Stones|GetStones_3))
  (Default|TurnOffFlame (Variables|Stones|GetStones_4))
  (Default|TurnOffFlame (Variables|Stones|GetStones_5)))

(event EventBeginPlay)

(event Collision|EventActorBeginOverlap
  (params (OtherActor :type Actor%20Object%20Reference)))

(event EventTick
  (params (DeltaSeconds :type Float%20%28single-precision%29)))

(fn ConstructionScript)