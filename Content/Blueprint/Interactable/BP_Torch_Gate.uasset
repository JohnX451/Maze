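; Interactable torch that the player lights with oil to open a gate.
; On begin play it caches the player character; Use works only if the player has oil and the torch is not yet active.
; Lighting it starts the flame effect and audio, clears the mesh's interaction tag and custom-depth highlight, spends oil, and calls OpenGate on the referenced gate.
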(event EventUse
  (bind _staticmesh (Variables|Default|GetStaticMesh))
  (if (and (> (Variables|/Game/Blueprint/Player/BP_PlayerCharacter.BP_PlayerCharacter_C|GetOil (Variables|Default|GetPlayer)) 0.0) (not (Variables|Default|GetbIsActive)))
    (Audio|SpawnSoundAttached "/Game/Audio/SFX/Fire/Cue_Torch_Ignite.Cue_Torch_Ignite" (Variables|Default|GetFlame) "None" "0, 0, 0" "0, 0, 0" "KeepRelativeOffset" false 1.0 1.0 0.0 0 0)
    (Components|Activation|SetActive (Variables|Default|GetAudio) true true)
    (Components|Activation|SetActive (Variables|Default|GetFlame) true true)
    (Variables|Default|SetbIsActive true)
    (Variables|/Script/Engine.ActorComponent|SetComponentTags _staticmesh (Utilities|Array|MakeArray "None"))
    (Rendering|SetRenderCustomDepth _staticmesh false)
    (Default|ChangeOil (Variables|Default|GetPlayer) -5.0 true)
    (Default|OpenGate (Variables|GameplayLogic|GetGate))))

(event EventBeginPlay
  (bind _asbp_player_character (Utilities|Casting|CastToBP_PlayerCharacter (Game|GetPlayerCharacter 0)))
  (Variables|Default|SetPlayer _asbp_player_character))

(fn ConstructionScript)