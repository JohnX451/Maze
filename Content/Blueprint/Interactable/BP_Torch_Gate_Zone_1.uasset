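; Interactable torch set for Zone 1 with five torches whose flames the player toggles with the Interact input.
; Each torch's collision box enables input and sets its selected flag on overlap, clearing the flag on exit.
; Interact passes the first selected torch's flame to ToggleFlame, which flips visibility but writes only Flame2Active, whichever torch is used.
; Torch 3's EnableInput receives no player controller, and no gate-opening logic is present.
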(event OnComponentBeginOverlap(Torch_2_Collision_Box)
  (params (OverlappedComponent :type Primitive%20Component%20Object%20Reference) (OtherActor :type Actor%20Object%20Reference) (OtherComp :type Primitive%20Component%20Object%20Reference) (OtherBodyIndex :type Integer) (bFromSweep :type Boolean) (SweepResult :type Hit%20Result%20Structure%20%28by%20ref%29))
  (Input|EnableInput (Game|GetPlayerController 0))
  (Variables|Selection|SetTorch_2_Selected true))

(event OnComponentEndOverlap(Torch_1_Collision_Box)
  (params (OverlappedComponent :type Primitive%20Component%20Object%20Reference) (OtherActor :type Actor%20Object%20Reference) (OtherComp :type Primitive%20Component%20Object%20Reference) (OtherBodyIndex :type Integer))
  ;[1 1 1] Activate and Deactivate Selection for Torch 1
  (Variables|Selection|SetTorch_1_Selected false))

(event OnComponentEndOverlap(Torch_2_Collision_Box)
  (params (OverlappedComponent :type Primitive%20Component%20Object%20Reference) (OtherActor :type Actor%20Object%20Reference) (OtherComp :type Primitive%20Component%20Object%20Reference) (OtherBodyIndex :type Integer))
  (Variables|Selection|SetTorch_2_Selected false))

(event OnComponentBeginOverlap(Torch_3_Collision_Box)
  (params (OverlappedComponent :type Primitive%20Component%20Object%20Reference) (OtherActor :type Actor%20Object%20Reference) (OtherComp :type Primitive%20Component%20Object%20Reference) (OtherBodyIndex :type Integer) (bFromSweep :type Boolean) (SweepResult :type Hit%20Result%20Structure%20%28by%20ref%29))
  (Input|EnableInput 0)
  (Variables|Selection|SetTorch_3_Selected true))

(event OnComponentEndOverlap(Torch_3_Collision_Box)
  (params (OverlappedComponent :type Primitive%20Component%20Object%20Reference) (OtherActor :type Actor%20Object%20Reference) (OtherComp :type Primitive%20Component%20Object%20Reference) (OtherBodyIndex :type Integer))
  (Variables|Selection|SetTorch_3_Selected false))

(event OnComponentBeginOverlap(Torch_4_Collision_Box)
  (params (OverlappedComponent :type Primitive%20Component%20Object%20Reference) (OtherActor :type Actor%20Object%20Reference) (OtherComp :type Primitive%20Component%20Object%20Reference) (OtherBodyIndex :type Integer) (bFromSweep :type Boolean) (SweepResult :type Hit%20Result%20Structure%20%28by%20ref%29))
  (Input|EnableInput (Game|GetPlayerController 0))
  (Variables|Selection|SetTorch_4_Selected true))

(event OnComponentEndOverlap(Torch_4_Collision_Box)
  (params (OverlappedComponent :type Primitive%20Component%20Object%20Reference) (OtherActor :type Actor%20Object%20Reference) (OtherComp :type Primitive%20Component%20Object%20Reference) (OtherBodyIndex :type Integer))
  (Variables|Selection|SetTorch_4_Selected false))

(event OnComponentBeginOverlap(Torch_5_Collision_Box)
  (params (OverlappedComponent :type Primitive%20Component%20Object%20Reference) (OtherActor :type Actor%20Object%20Reference) (OtherComp :type Primitive%20Component%20Object%20Reference) (OtherBodyIndex :type Integer) (bFromSweep :type Boolean) (SweepResult :type Hit%20Result%20Structure%20%28by%20ref%29))
  (Input|EnableInput (Game|GetPlayerController 0))
  (Variables|Selection|SetTorch_5_Selected true))

(event OnComponentEndOverlap(Torch_5_Collision_Box)
  (params (OverlappedComponent :type Primitive%20Component%20Object%20Reference) (OtherActor :type Actor%20Object%20Reference) (OtherComp :type Primitive%20Component%20Object%20Reference) (OtherBodyIndex :type Integer))
  (Variables|Selection|SetTorch_5_Selected false))

(event OnComponentBeginOverlap(Torch_1_Collision_Box)
  (params (OverlappedComponent :type Primitive%20Component%20Object%20Reference) (OtherActor :type Actor%20Object%20Reference) (OtherComp :type Primitive%20Component%20Object%20Reference) (OtherBodyIndex :type Integer) (bFromSweep :type Boolean) (SweepResult :type Hit%20Result%20Structure%20%28by%20ref%29))
  ;[1 1 1] Activate and Deactivate Selection for Torch 1
  (Input|EnableInput (Game|GetPlayerController 0))
  (Variables|Selection|SetTorch_1_Selected true))

(event EventBeginPlay
  (bind _asbp_player_character (Utilities|Casting|CastToBP_PlayerCharacter (Game|GetPlayerCharacter 0)))
  (Variables|Default|SetPlayer _asbp_player_character))

(event Input|ActionEvents|InputActionInteract
  (params (Key :type Key%20Structure :default "None"))
  (:Pressed
    (if (Variables|Selection|GetTorch_1_Selected)
      (CallFunction|ToggleFlame (Variables|Default|GetFlame_1) (Variables|Flames|GetFlame_1_Active))
      (elif (Variables|Selection|GetTorch_2_Selected)
        (CallFunction|ToggleFlame (Variables|Default|GetFlame_2) (Variables|Flames|GetFlame_2_Active))
        (elif (Variables|Selection|GetTorch_3_Selected)
          (CallFunction|ToggleFlame (Variables|Default|GetFlame_3) (Variables|Flames|GetFlame_3_Active))
          (elif (Variables|Selection|GetTorch_4_Selected)
            (CallFunction|ToggleFlame (Variables|Default|GetFlame_4) (Variables|Flames|GetFlame_4_Active))
            (elif (Variables|Selection|GetTorch_5_Selected)
              (CallFunction|ToggleFlame (Variables|Default|GetFlame_5) (Variables|Flames|GetFlame_5_Active)))))))))

(fn ConstructionScript)

(fn ToggleFlame
  (params (Flame :type Scene%20Component%20Object%20Reference) (CurrentState :type Boolean))
  (Development|SetHiddeninGame Flame CurrentState false)
  (Variables|Flames|SetFlame_2_Active (not CurrentState)))