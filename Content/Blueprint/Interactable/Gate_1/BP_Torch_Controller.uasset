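; Controller for a five-torch lights-out puzzle that opens a gate when every torch is lit.
; Zone entry initializes the torches in an alternating pattern and stops the monster; each interaction toggles the torch's linear neighbors.
; Solving it disables torch use and custom-depth rendering, opens the gate, then after a delay kills the flames and resumes the monster.
; All torches going out also resumes the monster, leaving the gate untouched.
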(event Custom|Torch%20Interacted
  (params (Torch :type BP%20Torch%20Gate%201%20Object%20Reference%20%28by%20ref%29))
  ;[1 1 1] Process Player Interaction with a Torch
  (CallFunction|ToggleFlameforSurrounding Torch)
  (if (CallFunction|AllTorchesLit)
    (CallFunction|DeactivateTorches)
    (Default|OpenGate (Variables|GamePlay|GetGate))
    (Utilities|FlowControl|Delay 8.0)
    (CallFunction|KillFlames)
    (Default|Resume (Variables|GamePlay|GetMonster) :!label _label)
    (elif (CallFunction|AllTorchesOff)
      (goto _label))))

(event Custom|Zone%20entered
  ;[1 1 1] Activate Flames for all Torches
  (Default|ZoneEntered (Variables|Torches|GetTorch_1) false)
  (Default|ZoneEntered (Variables|Torches|GetTorch_2) true)
  (Default|ZoneEntered (Variables|Torches|GetTorch_3) false)
  (Default|ZoneEntered (Variables|Torches|GetTorch_4) true)
  (Default|ZoneEntered (Variables|Torches|GetTorch_5) false)
  (Default|StopforPuzzle (Variables|GamePlay|GetMonster) (Transformation|GetActorLocation)))

(event EventBeginPlay)

(event Collision|EventActorBeginOverlap
  (params (OtherActor :type Actor%20Object%20Reference)))

(event EventTick
  (params (DeltaSeconds :type Float%20%28single-precision%29)))

(fn ConstructionScript)

(fn ToggleFlameforSurrounding
  (params (Center%20Torch :type BP%20Torch%20Gate%201%20Object%20Reference%20%28by%20ref%29))
  (if (== Center%20Torch (Variables|Torches|GetTorch_1))
    (Default|TogglefromOtherTorch (Variables|Torches|GetTorch_2))
    (elif (== Center%20Torch (Variables|Torches|GetTorch_2))
      (Default|TogglefromOtherTorch (Variables|Torches|GetTorch_1))
      (Default|TogglefromOtherTorch (Variables|Torches|GetTorch_3))
      (elif (== Center%20Torch (Variables|Torches|GetTorch_3))
        (Default|TogglefromOtherTorch (Variables|Torches|GetTorch_2))
        (Default|TogglefromOtherTorch (Variables|Torches|GetTorch_4))
        (elif (== Center%20Torch (Variables|Torches|GetTorch_4))
          (Default|TogglefromOtherTorch (Variables|Torches|GetTorch_3))
          (Default|TogglefromOtherTorch (Variables|Torches|GetTorch_5))
          (elif (== Center%20Torch (Variables|Torches|GetTorch_5))
            (Default|TogglefromOtherTorch (Variables|Torches|GetTorch_4))))))))

(fn AllTorchesLit
  (return (Math|Boolean|ANDBoolean (Variables|/Game/Blueprint/Interactable/Gate_1/BP_Torch_Gate_1.BP_Torch_Gate_1_C|GetbIsLit (Variables|Torches|GetTorch_1)) (Variables|/Game/Blueprint/Interactable/Gate_1/BP_Torch_Gate_1.BP_Torch_Gate_1_C|GetbIsLit (Variables|Torches|GetTorch_2)) (Variables|/Game/Blueprint/Interactable/Gate_1/BP_Torch_Gate_1.BP_Torch_Gate_1_C|GetbIsLit (Variables|Torches|GetTorch_3)) (Variables|/Game/Blueprint/Interactable/Gate_1/BP_Torch_Gate_1.BP_Torch_Gate_1_C|GetbIsLit (Variables|Torches|GetTorch_4)) (Variables|/Game/Blueprint/Interactable/Gate_1/BP_Torch_Gate_1.BP_Torch_Gate_1_C|GetbIsLit (Variables|Torches|GetTorch_5)))))

(fn AllTorchesOff
  (return (Math|Boolean|ANDBoolean (not (Variables|/Game/Blueprint/Interactable/Gate_1/BP_Torch_Gate_1.BP_Torch_Gate_1_C|GetbIsLit (Variables|Torches|GetTorch_1))) (not (Variables|/Game/Blueprint/Interactable/Gate_1/BP_Torch_Gate_1.BP_Torch_Gate_1_C|GetbIsLit (Variables|Torches|GetTorch_2))) (not (Variables|/Game/Blueprint/Interactable/Gate_1/BP_Torch_Gate_1.BP_Torch_Gate_1_C|GetbIsLit (Variables|Torches|GetTorch_3))) (not (Variables|/Game/Blueprint/Interactable/Gate_1/BP_Torch_Gate_1.BP_Torch_Gate_1_C|GetbIsLit (Variables|Torches|GetTorch_4))) (not (Variables|/Game/Blueprint/Interactable/Gate_1/BP_Torch_Gate_1.BP_Torch_Gate_1_C|GetbIsLit (Variables|Torches|GetTorch_5))))))

(fn DeactivateTorches
  (for _array_element (Utilities|Array|MakeArray (Variables|Torches|GetTorch_1) (Variables|Torches|GetTorch_2) (Variables|Torches|GetTorch_3) (Variables|Torches|GetTorch_4) (Variables|Torches|GetTorch_5))
    (Variables|/Game/Blueprint/Interactable/Gate_1/BP_Torch_Gate_1.BP_Torch_Gate_1_C|SetbIsUsable _array_element false)
    (Rendering|SetRenderCustomDepth (Variables|/Game/Blueprint/Interactable/Gate_1/BP_Torch_Gate_1.BP_Torch_Gate_1_C|GetStaticMesh _array_element) false)
    (Variables|/Script/Engine.ActorComponent|SetComponentTags (Variables|/Game/Blueprint/Interactable/Gate_1/BP_Torch_Gate_1.BP_Torch_Gate_1_C|GetStaticMesh _array_element) (Utilities|Array|MakeArray "None"))))

(fn KillFlames
  (for _array_element (Utilities|Array|MakeArray (Variables|Torches|GetTorch_1) (Variables|Torches|GetTorch_2) (Variables|Torches|GetTorch_3) (Variables|Torches|GetTorch_4) (Variables|Torches|GetTorch_5))
    (Components|Activation|SetActive (Variables|/Game/Blueprint/Interactable/Gate_1/BP_Torch_Gate_1.BP_Torch_Gate_1_C|GetFlame _array_element) false true)))