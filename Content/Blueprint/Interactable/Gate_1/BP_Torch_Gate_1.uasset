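; Interactable torch for the Gate 1 torch puzzle, with a flame the player can toggle on or off.
; On zone entry it takes an initial lit state, shows or hides the flame to match, tags its mesh as highlightable and becomes usable.
; Using it toggles the flame and notifies the Torch Controller; a separate event lets the center torch's effect toggle it without notifying.
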(event Custom|Toggle%20From%20Other%20Torch
  ;[1 1 1] Event if the Torch is affected by the center torch and needs to be toggled
  (CallFunction|ToggleFlame))

(event Custom|Zone%20Entered
  (params (InitialState :type Boolean))
  ;[1 1 1] Activate Torches when Player enters Zone. Set Flame to hidden except for specific active torches.
  (bind _output_get (Variables|Default|SetbIsLit InitialState))
  (Development|SetHiddeninGame (Variables|Default|GetFlame) (not _output_get) false)
  (Variables|/Script/Engine.ActorComponent|SetComponentTags (Variables|Default|GetStaticMesh) (Utilities|Array|MakeArray "highlightable"))
  (Variables|Default|SetbIsUsable true)
  (Components|Activation|SetActive (Variables|Default|GetFlame) true true))

(event EventUse
  ;[1 1 1] Interaction with Player. Toggle the Flame and notify Torch Controller.
  (if (Variables|Default|GetbIsUsable)
    (CallFunction|ToggleFlame)
    (Default|TorchInteracted (Variables|GameplayLogic|GetTorchController) self)))

(event EventBeginPlay
  (bind _asbp_player_character (Utilities|Casting|CastToBP_PlayerCharacter (Game|GetPlayerCharacter 0)))
  (Variables|Default|SetPlayer _asbp_player_character))

(fn ConstructionScript)

(fn ToggleFlame
  (Development|SetHiddeninGame (Variables|Default|GetFlame) (Variables|Default|GetbIsLit) false)
  (Variables|Default|SetbIsLit (not (Variables|Default|GetbIsLit))))