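; Procedural wall actor that lines a spline with deformed copies of one static mesh, built in the construction script.
; Each segment between spline points gets a mesh count from its length, with pieces evenly resized and doubled in number when stretched to 1.5 times MeshLength or more.
; Colliding spline mesh components follow the spline's positions and tangents, with tangents clamped to piece length.
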(event EventBeginPlay)

(event Collision|EventActorBeginOverlap
  (params (OtherActor :type Actor%20Object%20Reference)))

(event EventTick
  (params (DeltaSeconds :type Float%20%28single-precision%29)))

(fn ConstructionScript
  (bind _spline (Variables|Default|GetSpline))
  (bind _spline_2 (Variables|Default|GetSpline))
  ;[1 1 1] loop through segments
  (for _index (range 0 (- (Spline|GetNumberOfSplinePoints (Variables|Default|GetSpline)) 2))
    ;[1 1 1] get number of meshes in segment
    (bind _output_get (Variables|Default|SetCurrentSplineIndex _index))
    (Variables|Default|SetCurrentSplineDistance (Spline|GetDistanceAlongSplineatSplinePoint _spline_2 _output_get))
    (bind _output_get_2 (Variables|Default|SetCurrentSplineLength (- (Spline|GetDistanceAlongSplineatSplinePoint _spline_2 (+ _output_get 1)) (Spline|GetDistanceAlongSplineatSplinePoint _spline_2 _output_get))))
    (bind _output_get_3 (Variables|Default|SetCurrentSplineMeshes (/ _output_get_2 (Variables|Default|GetMeshLength))))
    (if (> _output_get_3 0)
      ;[1 1 1] mesh length adjusted for spline length, but below 50% of original length
      (bind _output_get_4 (Variables|Default|SetCorrectedMeshLength (/ (Variables|Default|GetCurrentSplineLength) (Variables|Default|GetCurrentSplineMeshes))))
      (if (< _output_get_4 (* (Variables|Default|GetMeshLength) 1.5))
        _
        (else
          (Variables|Default|SetCorrectedMeshLength (/ (Variables|Default|GetCorrectedMeshLength) 2.0))
          (Variables|Default|SetCurrentSplineMeshes (* (Variables|Default|GetCurrentSplineMeshes) 2))))
      (for _index_2 (range 0 (- (Variables|Default|GetCurrentSplineMeshes) 1))
        (bind _returnvalue (AddComponent|AddSplineMeshComponent false))
        (Components|StaticMesh|SetStaticMesh _returnvalue (Variables|Default|GetStaticMesh))
        (Collision|SetCollisionEnabled _returnvalue "QueryAndPhysics")
        (Collision|SetCollisionObjectType _returnvalue "ECC_WorldStatic")
        (Collision|SetCollisionResponsetoChannel _returnvalue "ECC_Visibility" "ECR_Block")
        (SplineMesh|SetStartandEnd _returnvalue (Spline|GetLocationatDistanceAlongSpline _spline (+ (* _index_2 (Variables|Default|GetCorrectedMeshLength)) (Variables|Default|GetCurrentSplineDistance)) "Local") (Math|Vector|ClampVectorSize (Spline|GetTangentatDistanceAlongSpline _spline (+ (* _index_2 (Variables|Default|GetCorrectedMeshLength)) (Variables|Default|GetCurrentSplineDistance)) "Local") 1.0 (Variables|Default|GetCorrectedMeshLength)) (Spline|GetLocationatDistanceAlongSpline _spline (+ (* (+ _index_2 1) (Variables|Default|GetCorrectedMeshLength)) (Variables|Default|GetCurrentSplineDistance)) "Local") (Math|Vector|ClampVectorSize (Spline|GetTangentatDistanceAlongSpline _spline (+ (* (+ _index_2 1) (Variables|Default|GetCorrectedMeshLength)) (Variables|Default|GetCurrentSplineDistance)) "Local") 1.0 (Variables|Default|GetCorrectedMeshLength)) true :!class /Script/Engine.SplineMeshComponent)
        (Transformation|AttachComponentToComponent _returnvalue (Variables|Default|GetSpline) "None" "KeepRelative" "KeepRelative" "KeepRelative" true)))))