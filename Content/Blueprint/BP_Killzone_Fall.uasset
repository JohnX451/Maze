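; A killzone actor that kills the player when they fall into it.
; On BeginPlay it caches the BP_PlayerCharacter instance and reacts only when that actor overlaps it.
; A DoOnce plays a pain sound attached to the player's Face, then after a short delay calls the player's Death.
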(event Collision|EventActorBeginOverlap
  (params (OtherActor :type Actor%20Object%20Reference))
  (if (== OtherActor (Variables|Default|GetPlayer))
    (Utilities|FlowControl|DoOnce false
      (:Completed
        (Audio|SpawnSoundAttached "/Game/Audio/SFX/Player/Cue_Player_Pain.Cue_Player_Pain" (Variables|/Game/Blueprint/Player/BP_PlayerCharacter.BP_PlayerCharacter_C|GetFace (Variables|Default|GetPlayer)) "None" "0, 0, 0" "0, 0, 0" "KeepRelativeOffset" false 1.0 1.0 0.0 0 0)
        (Utilities|FlowControl|Delay 1.0)
        (Default|Death (Variables|Default|GetPlayer))))))

(event EventBeginPlay
  (bind _returnvalue (Actor|GetActorOfClass "/Game/Blueprint/Player/BP_PlayerCharacter.BP_PlayerCharacter_C"))
  (Variables|Default|SetPlayer _returnvalue))

(fn ConstructionScript)