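; Actor component that shows its owning actor as an icon on the minimap, relative to the player.
; After a short delay on BeginPlay, if usable, it creates the icon widget and attaches a helper SceneComponent to the player's root.
; Each tick it moves the helper to the owner's transform and feeds its relative location and yaw to the icon, avoiding manual transform math.
; It also exposes icon data and icon removal.
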(event EventBeginPlay
  (if (Variables|Default|GetbIsUsable)
    (Utilities|FlowControl|Delay 0.2)
    ;[1 1 1] Create Minimap Icon
    (bind _returnvalue (UserInterface|CreateWidget "/Game/Minimap/WBP_Minimap_Icon.WBP_Minimap_Icon_C"))
    (bind _output_get (Variables|Default|Setminimap_icon _returnvalue))
    (Default|ChangeIcon _output_get (Variables|Default|GetIcon))
    (Default|ChangeSize _output_get (Variables|Default|GetIcon%20Size))
    (UserInterface|Viewport|AddtoViewport _output_get 0)
    (bind _returnvalue_2 (Game|AddComponentbyClass (Components|GetOwner) "/Script/Engine.SceneComponent" false))
    (Variables|Default|Setcalc_helper _returnvalue_2)
    ;[1 1 1] Update Icon Position based on Players Location and Rotation
    (Transformation|AttachComponentToComponent (Variables|Default|Getcalc_helper) (Variables|/Script/Engine.Actor|GetRootComponent (Game|GetPlayerCharacter 0)) "None" "KeepWorld" "KeepWorld" "KeepWorld" true)))

(event EventTick
  (params (DeltaSeconds :type Float%20%28single-precision%29))
  (if (Variables|Default|GetbIsUsable)
    (CallFunction|UpdateIconPosition)))

(fn UpdateIconPosition
  (bind _returnvalue (Components|GetOwner))
  (bind _calc_helper (Variables|Default|Getcalc_helper))
  ;[1 1 1] Calculate Icon Position
  (bind _calc_helper_2 (Variables|Default|Getcalc_helper)
    (:then
      (Transformation|SetWorldLocationAndRotation _calc_helper_2 (Transformation|GetActorLocation _returnvalue) (Transformation|GetActorRotation _returnvalue) false false)
      (bind _minimap_icon (Variables|Default|Getminimap_icon)
        (:then
          (Default|UpdateIconLocation _minimap_icon (Math|Conversions|ToVector2D(Vector) (Variables|/Script/Engine.SceneComponent|GetRelativeLocation _calc_helper)) (.yaw (Variables|/Script/Engine.SceneComponent|GetRelativeRotation _calc_helper))))
        (:else)))
    (:else)))

(fn GetMapIconData
  (return (Transformation|GetActorLocation (Components|GetOwner)) (Variables|Default|GetIcon) (Variables|Default|GetIcon%20Size)))

(fn RemoveIcon
  (Widget|RemovefromParent (Variables|Default|Getminimap_icon)))